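; BP_Stone is the player-controlled physics stone for a stone-skipping mechanic.
; On BeginPlay it caches the WorldSettings actor and adds the IMC_StoneSkipping Enhanced Input mapping context to its player controller.
; Each Tick applies a mass-scaled custom gravity force to the Cylinder, using world gravity times a gravity scale.
; The IA_Skip input calls Skip, which adds SkipVelocity as a velocity-change impulse, with no contact or state check.
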(event `self.ReceiveBeginPlay`
  (`KismetSystemLibrary.PrintString` "Hello")
  (bind _outactors (`GameplayStatics.GetAllActorsOfClass` "/Script/Engine.WorldSettings"))
  (set `self.WorldSettings` (`|GetArrayItem` _outactors))
  (bind _asplayer_controller (cast `PlayerController` (`self.GetController`)))
  (`EnhancedInputSubsystemInterface.AddMappingContext` (pcsubsystem `EnhancedInputLocalPlayerSubsystem` _asplayer_controller) "/Game/Input/IMC_StoneSkipping.IMC_StoneSkipping" 0 (struct)))

(event `self.ReceiveTick`
  (params (DeltaSeconds :type "Float (single-precision)"))
  (bind _cylinder (`self.Cylinder`))
  (`PrimitiveComponent.AddForce` _cylinder (`KismetMathLibrary.MakeVector` 0.0 0.0 (* (`WorldSettings.GlobalGravityZ` (`self.WorldSettings`)) (`self.GravtiyScale`) (`PrimitiveComponent.GetMass` _cylinder))) "None" false))

(event `EnhancedInput|/Game/Input/IA_Skip`
  (params (ActionValue :type Boolean) (ElapsedSeconds :type "Float (double-precision)") (TriggeredSeconds :type "Float (double-precision)") (InputAction :type "InputAction Object Reference" :default "/Game/Input/IA_Skip.IA_Skip"))
  (:`Triggered`
    (`self.Skip`)))

(fn `Skip`
  (`PrimitiveComponent.AddImpulse` (`self.Cylinder`) (`self.SkipVelocity`) "None" true)
  (return))

(fn `UserConstructionScript`)